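; Melee enemy NPC that endlessly chases player 0, attacks on arrival and opens closed doors it overlaps.
; An AIMoveTo loop retries on failure; on success, a forward line trace gates a random attack montage.
; The montage's HitNotify re-traces before applying damage, and completion resumes the chase.
; When AC_HealthStats fires OnDead, the enemy ragdolls, disables capsule collision and is destroyed after a delay.
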(event `self.ReceiveBeginPlay`
  (`KismetSystemLibrary.DelayUntilNextTick`)
  (`|ExecutionSequence`
    (:`then_0`
      (`|AIMoveTo` self (0.0 0.0 0.0) (`GameplayStatics.GetPlayerCharacter` 0) 50.0 :!label _label
        (:`OnSuccess`
          (`self.Hit`))
        (:`OnFail`
          (`KismetSystemLibrary.DelayUntilNextTick` :!label _label_2)
          (goto _label))))))

(event `Hit`
  (bind _mesh (`self.Mesh`))
  (bind _mesh_2 (`self.Mesh`))
  (bind _returnvalue (`KismetMathLibrary.TransformLocation` (`KismetMathLibrary.MakeTransform` (0.0 0.0 100.0)) (`SceneComponent.K2_GetComponentLocation` _mesh)))
  (bind _returnvalue_2 (`KismetMathLibrary.TransformLocation` (`KismetMathLibrary.MakeTransform` (0.0 0.0 100.0)) (`SceneComponent.K2_GetComponentLocation` _mesh_2)))
  (if (not (`self.bIsDead`))
    (bind _outhit (`KismetSystemLibrary.LineTraceSingle` _returnvalue (+ _returnvalue (* (`KismetMathLibrary.GreaterGreater_VectorRotator` (`SceneComponent.GetForwardVector` _mesh) (struct :`Yaw` 90.0)) 150.0)) "TraceTypeQuery4"))
    (bind (_bblockinghit _binitialoverlap _time _distance _location _impactpoint _normal _impactnormal _physmat _hitactor) (`GameplayStatics.BreakHitResult` _outhit))
    (if _bblockinghit
      (bind _asbp_third_person_character (cast `/Game/GameSystem/ThirdPerson/Blueprints/BP_ThirdPersonCharacter` _hitactor)
        (:`then`
          (bind _notifyname (`|PlayMontage` (`self.Mesh`) (`KismetArrayLibrary.Array_Random` (`self.AttackAnimMontages`)))
            (:`OnCompleted`
              (goto _label))
            (:`OnNotifyBegin`
              (if (== _notifyname "HitNotify")
                (bind _outhit_2 (`KismetSystemLibrary.LineTraceSingle` _returnvalue_2 (+ _returnvalue_2 (* (`KismetMathLibrary.GreaterGreater_VectorRotator` (`SceneComponent.GetForwardVector` _mesh_2) (struct :`Yaw` 90.0)) 150.0)) "TraceTypeQuery4"))
                (bind (_bblockinghit_2 _binitialoverlap_2 _time_2 _distance_2 _location_2 _impactpoint_2 _normal_2 _impactnormal_2 _physmat_2 _hitactor_2) (`GameplayStatics.BreakHitResult` _outhit_2))
                (if _bblockinghit_2
                  (cast `/Game/GameSystem/ThirdPerson/Blueprints/BP_ThirdPersonCharacter` _hitactor_2)
                  (`GameplayStatics.ApplyDamage` _asbp_third_person_character 20.0))))))
        (:`CastFailed`
          (goto _label_2)))
      (else
        (goto _label_2)))))

(event `self.ReceiveActorBeginOverlap`
  (params (OtherActor :type "Actor Object Reference"))
  (bind _asbp_simple_door (cast `/Game/GameSystem/Interactables/BP_SimpleDoor` OtherActor :!label _label_3))
  (`KismetSystemLibrary.PrintString` "TRY")
  (if (not (`/Game/GameSystem/Interactables/BP_SimpleDoor.bIsOpen` _asbp_simple_door))
    (`/Game/GameSystem/Interactables/BP_Interactable.Interact` _asbp_simple_door (struct :`TagName` "Interactor.NPC") self)
    (`KismetSystemLibrary.Delay` 1.0)
    (if (not (`/Game/GameSystem/Interactables/BP_SimpleDoor.bIsOpen` _asbp_simple_door))
      (goto _label_3))))

(event `self.AC_HealthStats.OnDead`
  (bind _mesh (`self.Mesh`))
  ;[1 1 1] Death
  (set `self.bIsDead` true)
  (`PrimitiveComponent.SetSimulatePhysics` _mesh true)
  (`SkeletalMeshComponent.SetPhysicsBlendWeight` _mesh 1.0)
  (`PrimitiveComponent.SetCollisionEnabled` (`self.CapsuleComponent`) "NoCollision")
  (`KismetSystemLibrary.Delay` 30.0)
  (`self.K2_DestroyActor`))

(fn `Attack`
  (bind _outitem (`KismetArrayLibrary.Array_Random` (`self.AttackAnimations`)))
  (set `self.AttackAnimLength` (`AnimationAsset.GetPlayLength` _outitem))
  (`SkeletalMeshComponent.PlayAnimation` (`self.Mesh`) _outitem false))

(fn `UserConstructionScript`)