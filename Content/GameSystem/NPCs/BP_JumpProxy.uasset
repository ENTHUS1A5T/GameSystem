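; Nav link proxy that makes AI characters jump across a smart link to its destination.
; When the link is reached, it casts the agent to Character and computes a custom-arc projectile velocity from the character's location to the destination, shaped by JumpArc.
; After a short delay, it launches the character with that velocity scaled by the sum of base and spec modifiers, overriding existing velocity on all axes.
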(event `self.ReceiveSmartLinkReached`
  (params (Agent :type "Actor Object Reference") (Destination :type "Vector Structure (by ref)"))
  (bind _ascharacter (cast `Character` Agent))
  (bind _output_get (set `self.JumpCharacter` _ascharacter))
  (bind _outlaunchvelocity (`GameplayStatics.SuggestProjectileVelocity_CustomArc` (`self.K2_GetActorLocation` _output_get) Destination 0.0 (`self.Jump_Arc`)))
  (`KismetSystemLibrary.Delay` 0.2)
  (`Character.LaunchCharacter` (`self.JumpCharacter`) (* _outlaunchvelocity (+ (`self.Jump_BaseMod`) (`self.Jump_SpecMod`))) true true))

(fn `UserConstructionScript`)