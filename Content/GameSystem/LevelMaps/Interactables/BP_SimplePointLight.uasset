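; BP_SimplePointLight is an interactable point light that players or other logic can switch on and off.
; An Interaction event checks IsTurnedOn and calls TurnOn or TurnOff to flip the state.
; Both events set the flag, then share one SetVisibility call that applies it to the PointLight component without propagating to children.
; The construction script only runs the parent's.
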(event `self.Interaction`
  (if (`self.bIsTurnedOn`)
    (`self.TurnOff`)
    (else
      (`self.TurnOn`))))

(event `TurnOn`
  (set `self.bIsTurnedOn` true)
  (`SceneComponent.SetVisibility` (`self.PointLight`) (`self.bIsTurnedOn`) false :!label _label))

(event `TurnOff`
  (set `self.bIsTurnedOn` false)
  (goto _label))

(fn `UserConstructionScript`
  (`parent.UserConstructionScript`))