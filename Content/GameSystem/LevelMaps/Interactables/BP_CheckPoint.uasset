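; BP_CheckPoint is a one-shot checkpoint actor that saves the game when something begins overlapping its Cylinder component.
; The overlap, with no check on the overlapping actor, passes the checkpoint's location and rotation, the player's current HP and a custom level name to BP_ThirdPersonController's SavetoSaveGame.
; It then shows a "Game Saved" notification through the PlayerHUD's main widget and destroys itself.
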(event `self.Cylinder.OnComponentBeginOverlap`
  (params (OverlappedComponent :type "PrimitiveComponent Object Reference") (OtherActor :type "Actor Object Reference") (OtherComp :type "PrimitiveComponent Object Reference") (OtherBodyIndex :type Integer) (bFromSweep :type Boolean) (SweepResult :type "HitResult Structure (by ref)"))
  (bind (_returnvalue_location _returnvalue_rotation) (`KismetMathLibrary.BreakTransform` (`self.GetTransform`)))
  ;[1 1 1] Save Game
  (bind _asbp_third_person_controller (cast `/Game/GameSystem/ThirdPerson/Blueprints/BP_ThirdPersonController` (`GameplayStatics.GetPlayerController` 0)))
  (`/Game/GameSystem/ThirdPerson/Blueprints/BP_ThirdPersonController.SavetoSaveGame` _asbp_third_person_controller false (`KismetMathLibrary.MakeTransform` _returnvalue_location _returnvalue_rotation) (`/Game/GameSystem/ThirdPerson/Blueprints/AC_HealthStats.CurrentHP` (`/Game/GameSystem/ThirdPerson/Blueprints/BP_ThirdPersonCharacter.HealthStats` (cast `/Game/GameSystem/ThirdPerson/Blueprints/BP_ThirdPersonCharacter` (`GameplayStatics.GetPlayerCharacter` 0) :!pure true))) (`KismetTextLibrary.Conv_TextToString` (`self.CustomLevelName`)))
  ;[1 1 1] Notification
  (bind _asplayer_hud (cast `/Game/GameSystem/GeneralBlueprints/PlayerHUD` (`PlayerController.GetHUD` (`GameplayStatics.GetPlayerController` 0))))
  (`/Game/GameSystem/GeneralBlueprints/HUDWidgets/WB_MainPlayerHUD.ShowNotification` (`/Game/GameSystem/GeneralBlueprints/PlayerHUD.WB_MainPlayerHUDRef` _asplayer_hud) "Game Saved")
  ;[0.3281 0 0] SelfDestroy
  (`self.K2_DestroyActor`))

(fn `UserConstructionScript`)