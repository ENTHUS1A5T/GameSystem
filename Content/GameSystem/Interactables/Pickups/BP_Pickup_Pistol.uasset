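; BP_Pickup_Pistol is an interactable pickup that gives the player a pistol and its ammo.
; On Interaction, it casts player character 0 to BP_ThirdPersonCharacter, adds AmmoAmount to the ACPistol component's stock ammo, then calls Equip on that component.
; The graph does not destroy or hide the pickup afterward, and its BeginPlay, overlap and Tick events are disabled stubs.
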(event `/Game/GameSystem/Interactables/BP_Interactable.Interaction`
  (params (Interactor :type "GameplayTag Structure"))
  (bind _asbp_third_person_character (cast `/Game/GameSystem/ThirdPerson/Blueprints/BP_ThirdPersonCharacter` (`GameplayStatics.GetPlayerCharacter` 0)))
  (bind _ac_pistol (`/Game/GameSystem/ThirdPerson/Blueprints/BP_ThirdPersonCharacter.AC_Pistol` _asbp_third_person_character))
  (set `/Game/GameSystem/ThirdPerson/Blueprints/AC_Pistol.AmmoInStock` (+ (`self.AmmoAmount`) (`/Game/GameSystem/ThirdPerson/Blueprints/AC_Pistol.AmmoInStock` _ac_pistol)) _ac_pistol)
  (`/Game/GameSystem/ThirdPerson/Blueprints/AC_Pistol.Equip` _ac_pistol))

(fn `UserConstructionScript`
  (`parent.UserConstructionScript`))