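; Flashlight pickup actor that grants the player a flashlight through the interaction system.
; On Interaction, it casts the interactor to BP_ThirdPersonCharacter and sets the Equiped flag on that character's ACFlashLight component.
; It has no other active logic and does not remove itself after use.
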(event `/Game/GameSystem/Interactables/BP_Interactable.Interaction`
  (params (Interactor :type "GameplayTag Structure") (`Interactor(Character)` :type "Character Object Reference"))
  (bind _asbp_third_person_character (cast `/Game/GameSystem/ThirdPerson/Blueprints/BP_ThirdPersonCharacter` `Interactor(Character)`))
  (set `/Game/GameSystem/ThirdPerson/Blueprints/AC_FlashLight.Equiped` true (`/Game/GameSystem/ThirdPerson/Blueprints/BP_ThirdPersonCharacter.AC_FlashLight` _asbp_third_person_character)))

(fn `UserConstructionScript`
  (`parent.UserConstructionScript`))