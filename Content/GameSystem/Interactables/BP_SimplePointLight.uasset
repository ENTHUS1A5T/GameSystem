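; BP_SimplePointLight is an interactable point light that is switched on and off through interaction.
; The Interaction event checks the IsTurnedOn flag and calls either TurnOn or TurnOff.
; Both events update the flag, then share one SetVisibility call that applies it to the PointLight without propagating to children.
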(event `self.Interaction`
  (params (Interactor :type "GameplayTag Structure"))
  (if (`self.bIsTurnedOn`)
    (`self.TurnOff`)
    (else
      (`self.TurnOn`))))

(event `TurnOn`
  (set `self.bIsTurnedOn` true)
  (`SceneComponent.SetVisibility` (`self.PointLight`) (`self.bIsTurnedOn`) false :!label _label))

(event `TurnOff`
  (set `self.bIsTurnedOn` false)
  (goto _label))

(fn `UserConstructionScript`
  (`parent.UserConstructionScript`))