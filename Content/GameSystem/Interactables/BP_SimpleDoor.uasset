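; Interactable swinging door that the player character opens and closes when interacting while overlapping its box.
; On opening, a dot product of the player's forward vector and the DoorOpenLocation arrow's forward vector picks the swing direction.
; The OpenDoorTime timeline drives the door mesh's relative yaw, playing from start to open and reversing from end to close.
; A busy flag ignores further interactions until the timeline finishes and toggles the open state.
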(event `self.Interaction`
  (params (Interactor :type "GameplayTag Structure"))
  (bind _asbp_third_person_character (cast `/Game/GameSystem/ThirdPerson/Blueprints/BP_ThirdPersonCharacter` (`GameplayStatics.GetPlayerCharacter` 0) :!pure true))
  (if (`PrimitiveComponent.IsOverlappingActor` (`self.Box`) _asbp_third_person_character)
    (if (`self.bIsInteractingDoor`)
      _
      (elif (`self.bIsOpen`)
        (set `self.bIsInteractingDoor` true)
        (bind (_direction _openangle) (`Timeline|OpenDoorTime` :!via `ReverseFromEnd` :!label _label)
          (:`Update`
            (`SceneComponent.K2_SetRelativeRotation` (`self.SM_Door`) (`KismetMathLibrary.MakeRotator` 0.0 0.0 (* _openangle (`self.DoorOpenSide`))) false false))
          (:`Finished`
            (set `self.bIsOpen` (not (`self.bIsOpen`)))
            (set `self.bIsInteractingDoor` false)))
        (else
          (if (> (`KismetMathLibrary.Dot_VectorVector` (`self.GetActorForwardVector` _asbp_third_person_character) (`SceneComponent.GetForwardVector` (`self.DoorOpenLocation`))) 0.0)
            (set `self.DoorOpenSide` 1.0)
            (else
              (set `self.DoorOpenSide` -1.0)))
          (set `self.bIsInteractingDoor` true)
          (goto _label :!via `PlayFromStart`))))))

(fn `UserConstructionScript`
  (`parent.UserConstructionScript`))